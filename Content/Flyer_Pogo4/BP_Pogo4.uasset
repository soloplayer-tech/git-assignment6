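; Player-controlled physics flyer that thrusts along its up axis and steers with pitch, bank and yaw torque, shown by spinning, glowing wheels.
; An altitude curve scales thrust, air resistance against a random wind set at BeginPlay, and audio volume.
; Tick eases camera angle, wheel glow and angular damping.
; Impacts play throttled sounds and, at speed, add random spin unless tagged NoChaos; gamepad buttons handle rear view, recentering and pause.
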(event OnComponentHit(Frame)
  (params (HitComponent :type Primitive%20Component%20Object%20Reference) (OtherActor :type Actor%20Object%20Reference) (OtherComp :type Primitive%20Component%20Object%20Reference) (NormalImpulse :type Vector :default "0, 0, 0") (Hit :type Hit%20Result%20Structure%20%28by%20ref%29))
  (bind (_bblockinghit _binitialoverlap _time _distance _location _impactpoint _normal _impactnormal _physmat _hitactor _hitcomponent) (Collision|BreakHitResult Hit))
  (bind _velocityvectorlength (Variables|Default|GetVelocityVectorLength))
  (bind _frame (Variables|Default|GetFrame))
  (bind _velocitysoundmodifier (Variables|Default|GetVelocitySoundModifier))
  (bind _collisionchaosmod (Variables|Default|GetCollisionChaosMod))
  (bind _returnvalue (* _velocityvectorlength _collisionchaosmod))
  (bind _returnvalue_2 (* _returnvalue -1.0))
  ;[1 1 1] Impact Sounds
  (if (> _velocitysoundmodifier 0.005)
    (Utilities|FlowControl|Sequence
      (:then_0
        (Utilities|FlowControl|DoOnce false :!label _label
          (:Completed
            (Audio|SpawnSoundatLocation "/Game/Flyer_Pogo4/Pogo4_Sounds/ImpactSounds/SndCue_Impact.SndCue_Impact" _location "0, 0, 0" (Math|Float|Lerp 0.05 12.0 _velocitysoundmodifier) (Math|Random|RandomFloatinRange 0.5 1.5) 0.0 0 0)
            ;[1 1 1] Collision  Randomized  Spin
            (if (not (Components|ComponentHasTag _hitcomponent "NoChaos"))
              (if (> _velocityvectorlength 2e+03)
                (Class|PrimitiveComponent|SetAngularDamping _frame 0.0)
                (Class|PrimitiveComponent|AddAngularImpulseinDegrees _frame (Math|Vector|MakeVector (Math|Random|RandomFloatinRange _returnvalue_2 _returnvalue) (Math|Random|RandomFloatinRange _returnvalue_2 _returnvalue) (Math|Random|RandomFloatinRange _returnvalue_2 _returnvalue)) "None" true))))))
      (:then_1
        (Utilities|FlowControl|Delay (Math|Random|RandomFloatinRange 0.05 0.19))
        (goto _label Reset)))))

(event EventBeginPlay
  (bind _wind_obj (Variables|Default|GetWind_Obj))
  ;[1 1 1] Set Intitial Camera
  (Components|Activation|SetActive (Variables|Default|GetCameraMain) true false)
  (Components|Activation|SetActive (Variables|Default|GetCameraReverse) false false)
  ;[1 1 1] Wind  Direction  and  Speed
  (Transformation|SetWorldRotation _wind_obj (Math|Rotator|MakeRotator 0.0 0.0 (Math|Random|RandomFloatinRange 0.0 359.98999)) false false)
  (Variables|Default|SetWind_Vec (* (Math|Vector|GetForwardVector _wind_obj) (Math|Random|RandomFloatinRange 1e+02 1.2e+03))))

(event EventTick
  (params (DeltaSeconds :type Float%20%28single-precision%29))
  (bind _wind_003_loop (Variables|Default|GetWind_003_loop))
  (bind _frame (Variables|Default|GetFrame))
  (bind _frame_2 (Variables|Default|GetFrame))
  (bind _returnvalue (Transformation|GetComponentVelocity _frame_2))
  (bind _returnvalue_2 (Class|PrimitiveComponent|GetAngularDamping _frame))
  (bind _returnvalue_3 (Math|Vector|VectorLength _returnvalue))
  ;[1 1 1] Air Resistance
  (Physics|AddForce _frame_2 (* (- _returnvalue (Variables|Default|GetWind_Vec)) (* (Variables|Default|GetAirResistance) (Math|Curves|GetFloatValue (Variables|Default|GetCrv_Bat_Atmos) (.z (Transformation|GetSocketLocation (Variables|Default|GetFrame) "None"))))) "None" true)
  ;[1 1 1] VelocitySoundMod  for  Volume
  (bind _output_get (Variables|Default|SetVelocitySoundModifier (Math|Float|NormalizetoRange (Math|Float|Clamp(Float) _returnvalue_3 0.0 2e+04) 0.0 2e+04)))
  (Variables|Default|SetVelocityVectorLength _returnvalue_3)
  ;[1 1 1] Rushing  Air
  (Audio|Components|Audio|SetVolumeMultiplier _wind_003_loop (Math|Float|Lerp 0.0 0.85 (* _output_get (Math|Curves|GetFloatValue (Variables|Default|GetCrv_Bat_Atmos) (.z (Transformation|GetSocketLocation (Variables|Default|GetFrame) "None"))))) :!class /Script/Engine.AudioComponent)
  (Audio|Components|Audio|SetPitchMultiplier _wind_003_loop (Math|Float|Lerp 0.2 1.5 _output_get))
  ;[0 0.304 1] Camera-Easing
  (bind _output_get_2 (Variables|Default|SetCameraAngle (+ (* (- (Variables|Default|GetCameraTargetAngle) (Variables|Default|GetCameraAngle)) 0.05) (Variables|Default|GetCameraAngle))))
  (Transformation|SetRelativeRotation (Variables|Default|GetSpringArmForward) (Math|Rotator|MakeRotator 0.0 _output_get_2 0.0) false false)
  (Transformation|SetRelativeRotation (Variables|Default|GetSpringArmReverse) (Math|Rotator|MakeRotator 0.0 _output_get_2 1.8e+02) false false)
  ;[1 1 1] Angular  Damping  Easing
  (Class|PrimitiveComponent|SetAngularDamping _frame (+ (* (- (Variables|Default|GetAngularDampingTarget) _returnvalue_2) 0.02) _returnvalue_2))
  ;[1 1 1] Glow  Pitch
  (bind _output_get_3 (Variables|Default|SetGlowPitch_Result (+ (* (- (Variables|Default|GetGlowPitch_Target) (Variables|Default|GetGlowPitch_Result)) 0.15) (Variables|Default|GetGlowPitch_Result))))
  (Rendering|Material|SetScalarParameterValueonMaterials (Variables|Default|GetWheel_Pitch) "Glow" (* _output_get_3 2.0))
  ;[1 1 1] Glow  Bank
  (bind _output_get_4 (Variables|Default|SetGlowBank_Result (+ (* (- (Variables|Default|GetGlowBank_Target) (Variables|Default|GetGlowBank_Result)) 0.15) (Variables|Default|GetGlowBank_Result))))
  (Rendering|Material|SetScalarParameterValueonMaterials (Variables|Default|GetWheel_Bank) "Glow" (* _output_get_4 2.0))
  ;[1 1 1] Glow  Yaw
  (bind _output_get_5 (Variables|Default|SetGlowYaw_Result (+ (* (- (Variables|Default|GetGlowYaw_Target) (Variables|Default|GetGlowYaw_Result)) 0.15) (Variables|Default|GetGlowYaw_Result))))
  (Rendering|Material|SetScalarParameterValueonMaterials (Variables|Default|GetWheel_Yaw) "Glow" (* _output_get_5 2.0)))

(event Input|AxisEvents|InputAxisFlyerThrustUpDn
  (params (AxisValue :type Float%20%28single-precision%29))
  (bind _returnvalue (Math|Float|Clamp(Float) AxisValue -1.0))
  (bind _crv_bat_throttle (Variables|Default|GetCrv_Bat_Throttle))
  (bind _crv_bat_atmos (Variables|Default|GetCrv_Bat_Atmos))
  (bind _snd_engine (Variables|Default|GetSnd_Engine))
  (bind _frame (Variables|Default|GetFrame))
  (bind _returnvalue_2 (Transformation|GetWorldLocation _frame))
  (bind _returnvalue_3 (Math|Curves|GetFloatValue _crv_bat_throttle _returnvalue))
  (bind _returnvalue_4 (Math|Float|Absolute(Float) _returnvalue_3))
  (bind _returnvalue_5 (Math|Curves|GetFloatValue _crv_bat_atmos (.z _returnvalue_2)))
  ;[1 1 1] Craft Movement
  (Physics|AddForce _frame (* (Math|Vector|GetUpVector (Variables|Default|GetFrame)) (* _returnvalue_3 (Variables|Default|GetThrustPower) _returnvalue_5)) "None" true)
  ;[1 1 1] Engine  Sound
  (Audio|Components|Audio|SetVolumeMultiplier _snd_engine (Math|Float|Lerp 0.0 0.7 (* _returnvalue_4 _returnvalue_5)) :!class /Script/Engine.AudioComponent)
  (Audio|Components|Audio|SetPitchMultiplier _snd_engine (Math|Float|Lerp 0.001 0.01 _returnvalue_4))
  (bind _output_get (Variables|Default|SetEngineGlow _returnvalue_4))
  ;[1 1 1] Engine  Glow
  (Rendering|Material|SetScalarParameterValueonMaterials (Variables|Default|GetFrame) "Glow" _output_get)
  ;[1 1 1] Thrust  Visiblity
  (Rendering|Material|SetScalarParameterValueonMaterials (Variables|Default|GetFrame) "Glow" (* _output_get (Math|Curves|GetFloatValue (Variables|Default|GetCrv_Bat_Atmos) (.z (Transformation|GetWorldLocation (Variables|Default|GetFrame)))))))

(event Input|AxisEvents|InputAxisCameraUpDn
  (params (AxisValue :type Float%20%28single-precision%29))
  ;[1 1 1] CameraAngle
  (Variables|Default|SetCameraTargetAngle (Math|Float|Clamp(Float) (+ (* (Math|Float|Clamp(Float) AxisValue -1.0) 1.0) (Variables|Default|GetCameraTargetAngle)) -7e+01 7e+01)))

(event Input|AxisEvents|InputAxisFlyerPitchUpDn
  (params (AxisValue :type Float%20%28single-precision%29))
  (bind _returnvalue (Math|Float|Clamp(Float) AxisValue -1.0))
  (bind _frame (Variables|Default|GetFrame))
  (bind _crv_bat_torque (Variables|Default|GetCrv_Bat_Torque))
  (bind _returnvalue_2 (Math|Curves|GetFloatValue _crv_bat_torque _returnvalue))
  ;[1 1 1] Craft Movement
  (Class|PrimitiveComponent|AddTorqueinDegrees _frame (* (Math|Vector|GetRightVector _frame) (* _returnvalue_2 (Variables|Default|GetTorquePower))) "None" true)
  (Variables|Default|SetGlowPitch_Target (Math|Float|Absolute(Float) _returnvalue_2))
  ;[1 1 1] Torque - Wheel  Rotation : Pitch
  (Transformation|AddLocalRotation (Variables|Default|GetWheel_Pitch) (Math|Rotator|MakeRotator 0.0 (* _returnvalue_2 2e+01) 0.0) false false))

(event Input|AxisEvents|InputAxisFlyerBankRightLeft
  (params (AxisValue :type Float%20%28single-precision%29))
  (bind _returnvalue (Math|Float|Clamp(Float) AxisValue -1.0))
  (bind _crv_bat_throttle (Variables|Default|GetCrv_Bat_Throttle))
  (bind _frame (Variables|Default|GetFrame))
  (bind _returnvalue_2 (Math|Curves|GetFloatValue _crv_bat_throttle _returnvalue))
  ;[1 1 1] Craft Movement
  (Class|PrimitiveComponent|AddTorqueinDegrees _frame (* (Math|Vector|GetForwardVector _frame) (* _returnvalue_2 (Variables|Default|GetTorquePower))) "None" true)
  (Variables|Default|SetGlowBank_Target (Math|Float|Absolute(Float) _returnvalue_2))
  ;[1 1 1] Torque - Wheel  Rotation : Bank
  (Transformation|AddLocalRotation (Variables|Default|GetWheel_Bank) (Math|Rotator|MakeRotator (* _returnvalue_2 12.0) 0.0 0.0) false false))

(event Input|AxisEvents|InputAxisFlyerYawRightLeft
  (params (AxisValue :type Float%20%28single-precision%29))
  (bind _returnvalue (Math|Float|Clamp(Float) AxisValue -1.0))
  (bind _crv_bat_torque (Variables|Default|GetCrv_Bat_Torque))
  (bind _frame (Variables|Default|GetFrame))
  (bind _returnvalue_2 (Math|Curves|GetFloatValue _crv_bat_torque _returnvalue))
  ;[1 1 1] Craft Movement
  (Class|PrimitiveComponent|AddTorqueinDegrees _frame (* (Math|Vector|GetUpVector _frame) (* _returnvalue_2 (* (Variables|Default|GetTorquePower) 1.0))) "None" true)
  (Variables|Default|SetGlowYaw_Target (Math|Float|Absolute(Float) _returnvalue_2))
  ;[1 1 1] Torque - Wheel  Rotation : Yaw
  (Transformation|AddLocalRotation (Variables|Default|GetWheel_Yaw) (Math|Rotator|MakeRotator 0.0 0.0 (* _returnvalue_2 -16.0)) false false))

(event Input|GamepadEvents|GamepadRightThumbstick
  (params (Key :type Key%20Structure))
  ;[1 1 1] Re-Center Camera
  (:Pressed
    (Variables|Default|SetCameraTargetAngle 0.0)))

(event Input|GamepadEvents|GamepadSpecialRight
  (params (Key :type Key%20Structure))
  ;[1 1 1] Pause
  (:Pressed
    (if (Game|IsGamePaused)
      (Game|SetGamePaused false)
      (else
        (Game|SetGamePaused true)))))

(event Input|GamepadEvents|GamepadLeftShoulder
  (params (Key :type Key%20Structure))
  (bind _cameramain (Variables|Default|GetCameraMain))
  (bind _camerareverse (Variables|Default|GetCameraReverse))
  ;[1 1 1] Camera  Rear-View
  (:Pressed
    (Components|Activation|SetActive _camerareverse true false)
    (Components|Activation|SetActive _cameramain false false))
  (:Released
    (Components|Activation|SetActive _cameramain true false)
    (Components|Activation|SetActive _camerareverse false false)))

(event Input|GamepadEvents|GamepadRightShoulder
  (params (Key :type Key%20Structure))
  (bind _cameramain (Variables|Default|GetCameraMain))
  (bind _camerareverse (Variables|Default|GetCameraReverse))
  ;[1 1 1] Camera  Rear-View
  (:Pressed
    (Components|Activation|SetActive _camerareverse true false)
    (Components|Activation|SetActive _cameramain false false))
  (:Released
    (Components|Activation|SetActive _cameramain true false)
    (Components|Activation|SetActive _camerareverse false false)))

(fn ConstructionScript)